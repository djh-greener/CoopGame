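; Speed-up powerup buff that temporarily doubles a player's walk speed.
; TickBuff sets the CharacterMovementComponent's MaxWalkSpeed to twice its current max speed, waits a few seconds, then sets it to half of the then-current value.
; Both changes scale GetMaxSpeed, which depends on movement mode, rather than restoring a saved value, and each prints the new speed.
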(event EventBeginPlay)

(event Collision|EventActorBeginOverlap
  (params (OtherActor :type Actor%20Object%20Reference)))

(event EventTick
  (params (DeltaSeconds :type Float%20%28single-precision%29)))

(event EventTickBuff
  (params (Player :type S%20Character%20Object%20Reference))
  (bind _returnvalue (Actor|GetComponentbyClass Player "/Script/Engine.CharacterMovementComponent"))
  (bind _returnvalue_2 (Class|MovementComponent|GetMaxSpeed _returnvalue))
  (bind _output_get (Variables|/Script/Engine.CharacterMovementComponent|SetMaxWalkSpeed _returnvalue (* _returnvalue_2 2.0)))
  (Development|PrintString (Utilities|String|ToString(Float) _output_get))
  (Utilities|FlowControl|Delay 3.0)
  (bind _output_get_2 (Variables|/Script/Engine.CharacterMovementComponent|SetMaxWalkSpeed _returnvalue (* _returnvalue_2 0.5)))
  (Development|PrintString (Utilities|String|ToString(Float) _output_get_2)))

(fn ConstructionScript)