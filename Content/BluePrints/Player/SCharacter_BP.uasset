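; Player character Blueprint that adds the local HUD and handles camera zoom.
; On BeginPlay, only when locally controlled, it creates the crosshair and health indicator widgets and adds them to the viewport.
; BeginZoom and EndZoom play and reverse a single Timeline that drives the camera component's field of view and relative location for a smooth transition in and out.
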(event EventBeginPlay
  (bind _returnvalue (Game|GetPlayerController 0))
  (if (Pawn|IsLocallyControlled)
    (Utilities|FlowControl|Sequence
      (:then_0
        (bind _returnvalue_2 (UserInterface|CreateWidget "/Game/BluePrints/UI/WBP_Crosshair.WBP_Crosshair_C" _returnvalue))
        (UserInterface|Viewport|AddtoViewport _returnvalue_2 0))
      (:then_1
        (bind _returnvalue_3 (UserInterface|CreateWidget "/Game/BluePrints/UI/WBP_HealthIndicator.WBP_HealthIndicator_C" _returnvalue))
        (UserInterface|Viewport|AddtoViewport _returnvalue_3 0)))))

(event EventBeginZoom
  (bind _cameracomp (Variables|Default|GetCameraComp))
  (bind (_direction _fov _rl) (Timeline|Timeline Play)
    (:Update
      (Utilities|FlowControl|Sequence
        (:then_0
          (Camera|SetFieldOfView _cameracomp _fov))
        (:then_1
          (Transformation|SetRelativeLocation _cameracomp _rl false false))))))

(event EventEndZoom
  (bind _cameracomp (Variables|Default|GetCameraComp))
  (bind (_direction _fov _rl) (Timeline|Timeline Reverse)
    (:Update
      (Utilities|FlowControl|Sequence
        (:then_0
          (Camera|SetFieldOfView _cameracomp _fov))
        (:then_1
          (Transformation|SetRelativeLocation _cameracomp _rl false false))))))

(fn ConstructionScript)