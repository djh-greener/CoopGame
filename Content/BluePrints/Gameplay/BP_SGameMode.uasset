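; Game mode Blueprint that spawns tracer bots and rewards the players who kill them.
; SpawnNewBot runs an EQS query for a random spawn location from the best 25%, then spawns BP_TracerBot at the returned results, adjusting for collision.
; An actor-killed delegate bound at BeginPlay adds a fixed score to the killer's SPlayerState when the victim is a tracer bot.
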(event Custom|OnQueryFinishedEvent_Event_0
  (params (QueryInstance :type Env%20Query%20Instance%20Blueprint%20Wrapper%20Object%20Reference) (QueryStatus :type EEnvQueryStatus%20Enum :default "Processing"))
  (switch Utilities|FlowControl|Switch|SwitchonEEnvQueryStatus QueryStatus
    (:Success
      (bind _resultlocations (AI|EQS|GetQueryResultsasLocations QueryInstance))
      (for _array_element _resultlocations
        (Game|SpawnActorfromClass "/Game/TracerBot/BP_TracerBot.BP_TracerBot_C" (Math|Transform|MakeTransform _array_element) "AdjustIfPossibleButDontSpawnIfColliding" 0 0)))))

(event Custom|OnActorKilled_Event_0
  (params (VictimActor :type Actor%20Object%20Reference) (KillerActor :type Actor%20Object%20Reference) (KillerController :type Controller%20Object%20Reference))
  (bind _playerstate (Variables|/Script/Engine.Controller|GetPlayerState KillerController))
  (Utilities|Casting|CastToSTracerBor VictimActor)
  (Utilities|IsValid _playerstate
    (:Is%20Valid
      (bind _assplayer_state (Utilities|Casting|CastToSPlayerState _playerstate))
      (Class|SPlayerState|AddScore _assplayer_state 2e+01))))

(event EventBeginPlay
  (EventDispatchers|AssignOnActorKilled (delegate Custom|OnActorKilled_Event_0)))

(event EventSpawnNewBot
  (bind _returnvalue (AI|EQS|RunEQSQuery "/Game/BluePrints/EQS/EQS_FindSpawnLocation.EQS_FindSpawnLocation" self "RandomBest25Pct"))
  (EventDispatchers|AssignOnQueryFinishedEvent _returnvalue (delegate Custom|OnQueryFinishedEvent_Event_0)))

(fn ConstructionScript)